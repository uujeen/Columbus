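; BP_Stamp is a collectible stamp pickup whose Cylinder spins on roll by a fixed step every tick.
; Any overlap with its Box lowers StampCount on BP_ColumbusGS, raises Stamps on player 0's BP_ColumbusPC, then destroys the actor.
; The overlap checks neither the overlapping actor nor network authority.
; An uncalled WhichComputer macro branches by server or client, and a stray SpawnActor node never runs.
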(event OnComponentBeginOverlap(Box)
  (params (OverlappedComponent :type Primitive%20Component%20Object%20Reference) (OtherActor :type Actor%20Object%20Reference) (OtherComp :type Primitive%20Component%20Object%20Reference) (OtherBodyIndex :type Integer) (bFromSweep :type Boolean) (SweepResult :type Hit%20Result%20Structure%20%28by%20ref%29))
  (bind _asbp_columbus_gs (Utilities|Casting|CastToBP_ColumbusGS (Game|GetGameState)))
  (Math|Integer|DecrementInt (Variables|/Game/ThirdPerson/Blueprints/BP_ColumbusGS.BP_ColumbusGS_C|GetStampCount _asbp_columbus_gs)
    (:%20%20
      (bind _asbp_columbus_pc (Utilities|Casting|CastToBP_ColumbusPC (Game|GetPlayerController 0)))
      (Math|Integer|IncrementInt (Variables|/Game/ThirdPerson/Blueprints/BP_ColumbusPC.BP_ColumbusPC_C|GetStamps _asbp_columbus_pc)
        (:%20%20
          (Actor|DestroyActor))))))

(event EventTick
  (params (DeltaSeconds :type Float%20%28single-precision%29))
  (bind _cylinder (Variables|Default|GetCylinder))
  (bind _relativerotation (Variables|/Script/Engine.SceneComponent|GetRelativeRotation _cylinder))
  (Transformation|SetRelativeRotation _cylinder (Math|Rotator|MakeRotator (+ (.roll _relativerotation) 5.0) (.pitch _relativerotation) (.yaw _relativerotation)) false false))

(fn ConstructionScript)